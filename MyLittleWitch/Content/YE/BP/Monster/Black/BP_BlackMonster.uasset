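; Enemy monster Blueprint that chases the player, attacks by range and shows its health through an HP widget.
; A looping timer measures player distance, choosing random melee montages up close or occasional cast montages from afar, otherwise resuming AIMoveTo.
; Separate events toggle fist collision for damage, launch the monster, trace hits and spawn ball or beam projectiles.
; Incoming damage triggers random flinch montages or a knockback death with particles before destruction.
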(event OnComponentBeginOverlap(Ham_Fist)
  (params (OverlappedComponent :type Primitive%20Component%20Object%20Reference) (OtherActor :type Actor%20Object%20Reference) (OtherComp :type Primitive%20Component%20Object%20Reference) (OtherBodyIndex :type Integer) (bFromSweep :type Boolean) (SweepResult :type Hit%20Result%20Structure%20%28by%20ref%29))
  ;[1 1 1] Fist Collision
  (if (== OtherActor (Game|GetPlayerCharacter 0))
    (CallFunction|DoDamage)
    ;;[1 1 1] Impulse
    (if (Variables|Default|GetIsAttacking)
      (Class|BPICharacter|GetHit(Message) OtherActor (Transformation|GetActorLocation)))))

(event Custom|Launcher
  (bind _charactermovement (Variables|Character|GetCharacterMovement))
  ;[1 1 1] Launch to Character
  (Variables|/Script/Engine.CharacterMovementComponent|SetGroundFriction _charactermovement 0.0)
  (Character|LaunchCharacter (+ (* (Transformation|GetActorForwardVector) (Variables|Default|GetLaunchForce)) (* (Transformation|GetActorUpVector) (Variables|Default|GetJumpForce))) false false)
  (Utilities|FlowControl|RetriggerableDelay 25.0)
  (Variables|/Script/Engine.CharacterMovementComponent|SetGroundFriction _charactermovement 8.0))

(event Custom|Seek%20Player
  ;[1 1 1] Seek Player
  ;;[1 1 1] Flinch
  (if (Variables|Default|GetAlive)
    (if (not (Variables|Default|GetFlinch))
      (if (Variables|Default|GetIsAttacking)
        (Components|Movement|StopMovementImmediately (Variables|Character|GetCharacterMovement))
        (else
          ;;[1 1 1] Radius
          (AI|AIMoveTo self "0, 0, 0" (Game|GetPlayerCharacter 0) 5e+02 false
            (:then
              _)
            (:OnSuccess
              _)
            (:OnFail
              _))
          (Utilities|FlowControl|Delay 0.2)
          (CallFunction|SeekPlayer))))))

(event Custom|Ham%20Down%20Trace
  (bind _ham_fist (Variables|Default|GetHam_Fist))
  (bind _returnvalue (Transformation|GetWorldLocation _ham_fist))
  ;[1 1 1] ATK_EF
  (bind _outhit (Collision|SphereTraceForObjects _returnvalue (+ _returnvalue (* (Math|Vector|GetForwardVector (Transformation|GetWorldRotation _ham_fist)) 2e+02)) 64.0 (Utilities|Array|MakeArray "ObjectTypeQuery3") false 0 "None"))
  (if (== (.HitActor (Collision|BreakHitResult _outhit)) (Game|GetPlayerCharacter 0))
    (bind _returnvalue_2 (Effects|SpawnEmitteratLocation "/Game/YE/BP/Monster/Black/P_Sevarog_DownATK.P_Sevarog_DownATK" (.Location (Collision|BreakHitResult _outhit))))
    (Transformation|SetWorldScale3D _returnvalue_2 "2.000000,2.000000,2.000000")))

(event Custom|Castball
  (bind _lt_fist (Variables|Default|GetLt_Fist))
  (bind _returnvalue (Transformation|GetWorldLocation _lt_fist))
  ;[1 1 1] Cast
  (Game|SpawnActorfromClass "/Game/YE/BP/Monster/Black/BP_CastBall.BP_Castball_C" (Math|Transform|MakeTransform _returnvalue (Math|Rotator|FindLookatRotation _returnvalue (Transformation|GetActorLocation (Game|GetPlayerCharacter 0)))) "Undefined" 0 0))

(event Custom|Do%20Damage
  ;[1 1 1] Do Damage
  (Game|Damage|ApplyDamage (Game|GetPlayerCharacter 0) (Variables|Default|GetMaxDamage) 0 self))

(event Custom|Distance%20Player
  ;[1 1 1] Check Distance
  ;;[1 1 1] Flinch
  (if (Variables|Default|GetAlive)
    (if (not (Variables|Default|GetFlinch))
      ;;[1 1 1] How Often
      (Utilities|Time|SetTimerbyFunctionName 0 "Player Distance" 1.0 true))))

(event Custom|Close%20Range
  ;[1 1 1] Attack
  (Variables|Default|SetIsAttacking true)
  (switch int (Math|Random|RandomIntegerinRange 0 1)
    (:0
      (Variables|Default|SetATK_Montage "/Game/YE/BP/Monster/Black/Animations/Swing1_Slow_Mon.Swing1_Slow_Mon")
      (Variables|Default|SetLaunchForce 2e+02 :!label _label)
      ;;[1 1 1] Damage
      (Variables|Default|SetMaxDamage 2e+02))
    (:1
      (Variables|Default|SetATK_Montage "/Game/YE/BP/Monster/Black/Animations/DownATK_Mon.DownATK_Mon")
      (Variables|Default|SetLaunchForce 4e+02)
      (Variables|Default|SetMaxDamage 4e+02))
    (:2
      (Variables|Default|SetATK_Montage "/Game/YE/BP/Monster/Black/Animations/Swing1_Slow_Mon.Swing1_Slow_Mon")
      (goto _label))
    (:3
      (Variables|Default|SetATK_Montage "/Game/YE/BP/Monster/Black/Animations/Swing1_Slow_Mon.Swing1_Slow_Mon")
      (goto _label)))
  (bind _returnvalue (Animation|PlayAnimMontage (Variables|Default|GetATK_Montage) 1.0 "None"))
  (Utilities|FlowControl|Delay _returnvalue)
  (Variables|Default|SetIsAttacking false)
  (CallFunction|SeekPlayer)
  ;[1 1 1] if Close  // Player Distance
  (if (not (>= (Variables|Default|GetDistance) 8.5e+02))
    (CallFunction|FacePlayer)))

(event Custom|Far%20Range
  ;[1 1 1] Attack
  (Variables|Default|SetIsAttacking true)
  (switch int (Math|Random|RandomIntegerinRange 0 1)
    (:0
      (Variables|Default|SetATK_Montage "/Game/YE/BP/Monster/Black/Animations/Cast_Mon.Cast_Mon"))
    (:1
      (Variables|Default|SetATK_Montage "/Game/YE/BP/Monster/Black/Animations/Point_Mon.Point_Mon")))
  (bind _returnvalue (Animation|PlayAnimMontage (Variables|Default|GetATK_Montage) 1.0 "None"))
  (Utilities|FlowControl|Delay _returnvalue)
  (Variables|Default|SetIsAttacking false)
  (CallFunction|SeekPlayer)
  ;[1 1 1] if Close  // Player Distance
  (if (not (>= (Variables|Default|GetDistance) 8.5e+02))
    (CallFunction|FacePlayer)))

(event Custom|Face%20Player
  ;[1 1 1] Face to Player
  (Transformation|SetActorRotation (Math|Rotator|FindLookatRotation (Transformation|GetActorLocation) (Transformation|GetActorLocation (Game|GetPlayerCharacter 0)))))

(event Custom|dCol%20Ham%20Fist
  ;[1 1 1] Fist Collision
  (Collision|SetCollisionEnabled (Variables|Default|GetHam_Fist) "NoCollision"))

(event Custom|Castbeam
  (bind _rt_fist (Variables|Default|GetRt_Fist))
  (bind _returnvalue (Transformation|GetWorldLocation _rt_fist))
  ;[1 1 1] Castbeam
  (Game|SpawnActorfromClass "/Game/YE/BP/Monster/Black/BP_CastBeam.BP_CastBeam_C" (Math|Transform|MakeTransform _returnvalue (Math|Rotator|FindLookatRotation _returnvalue (Transformation|GetActorLocation (Game|GetPlayerCharacter 0)))) "Undefined" 0 0))

(event Custom|Ham%20Trace
  (bind _hammer (Variables|Default|GetHammer))
  (bind _returnvalue (Transformation|GetWorldLocation _hammer))
  ;[1 1 1] ATK_EF
  (bind _outhit (Collision|SphereTraceForObjects _returnvalue (+ _returnvalue (* (Math|Vector|GetForwardVector (Transformation|GetWorldRotation _hammer)) 2e+02)) 64.0 (Utilities|Array|MakeArray "ObjectTypeQuery3") false 0 "None"))
  (if (== (.HitActor (Collision|BreakHitResult _outhit)) (Game|GetPlayerCharacter 0))
    (Development|PrintString "Hello")))

(event Custom|eCol%20Ham%20Fist
  ;[1 1 1] Fist Collision
  (Collision|SetCollisionEnabled (Variables|Default|GetHam_Fist) "QueryAndPhysics"))

(event EventBeginPlay
  ;[1 1 1] Base
  (Variables|Default|SetHealth (Variables|Default|GetMaxHealth))
  (bind _aswb_black_monster_hp (Utilities|Casting|CastToWB_BlackMonsterHP (UserInterface|GetUserWidgetObject (Variables|Default|GetHP%20Bar))))
  (Variables|/Game/YE/WB/WB_BlackMonsterHP.WB_BlackMonsterHP_C|SetHealthInterface _aswb_black_monster_hp self)
  (Variables|Default|SetAlive true)
  (Utilities|FlowControl|Delay 0.2)
  (CallFunction|SeekPlayer)
  (CallFunction|DistancePlayer))

(event Game|Damage|EventAnyDamage
  (params (Damage :type Float%20%28single-precision%29) (DamageType :type Damage%20Type%20Object%20Reference) (InstigatedBy :type Controller%20Object%20Reference) (DamageCauser :type Actor%20Object%20Reference))
  ;[1 1 1] Get Damage
  (if (!= DamageCauser self)
    (Variables|Default|SetDamage Damage)
    (bind _output_get (Variables|Default|SetHealth (- (Variables|Default|GetHealth) Damage)))
    (if (<= _output_get 0.0)
      (Pawn|Components|CharacterMovement|DisableMovement (Variables|Character|GetCharacterMovement))
      (bind _returnvalue (Animation|PlayAnimMontage "/Game/YE/BP/Monster/Black/Knock_back_Mon.Knock_back_Mon" 1.0 "None" :!label _label))
      (Utilities|FlowControl|Delay _returnvalue)
      (Effects|SpawnEmitterAttached "/Game/YE/BP/Monster/Black/P_Sub_Cast.P_Sub_Cast" (Variables|Character|GetMesh) "None" "0, 0, 0" "0, 0, 0" "3.000000,3.000000,3.000000")
      (Utilities|FlowControl|Delay 2.0)
      (Variables|Default|SetAlive false)
      (Utilities|FlowControl|Delay 0.2)
      (Actor|DestroyActor)
      (elif (>= (Variables|Default|GetDamage) 5.0)
        (Variables|Default|SetFlinch true)
        (switch int (Math|Random|RandomIntegerinRange 0 2)
          (:0
            (Variables|Default|SetATK_Montage "/Game/YE/BP/Monster/Red/Animations/Hit_Front_Mon.Hit_Front_Mon"))
          (:1
            (Variables|Default|SetATK_Montage "/Game/YE/BP/Monster/Red/Animations/Knock_Fwd_Mon.Knock_Fwd_Mon"))
          (:2
            (Variables|Default|SetATK_Montage "/Game/YE/BP/Monster/Red/Animations/Knock_Bwd_Mon.Knock_Bwd_Mon")))
        (bind _returnvalue_2 (Animation|PlayAnimMontage (Variables|Default|GetATK_Montage) 1.0 "None"))
        (Utilities|FlowControl|Delay _returnvalue_2)
        (Variables|Default|SetFlinch false)
        (if (<= (Variables|Default|GetHealth) 0.0)
          (goto _label))))))

(event EventDotDamage
  (params (Damage :type Float%20%28single-precision%29))
  ;[1 1 1] Dot damage 피격
  (if (not (Variables|Default|GetDot))
    (Variables|Default|SetDot true)
    (Variables|Default|SetHealth (- (Variables|Default|GetHealth) Damage))
    (bind _returnvalue (Animation|PlayAnimMontage self 0 1.0 "None"))
    (Utilities|FlowControl|Delay _returnvalue)
    (Variables|Default|SetDot false)))

(fn ConstructionScript)

(fn PlayerDistance
  ;[1 1 1] Distance
  (if (not (Variables|Default|GetIsAttacking))
    ;;[1 1 1] Detect
    (bind _output_get (Variables|Default|SetDistance (Math|Vector|VectorLength (- (Transformation|GetActorLocation) (Transformation|GetActorLocation (Game|GetPlayerCharacter 0))))))
    ;;[1 1 1] Far
    (if (>= _output_get 8.5e+02)
      (if (== (Math|Random|RandomIntegerinRange 0 4) 0)
        (CallFunction|FarRange)
        (else
          (CallFunction|SeekPlayer)))
      (else
        (CallFunction|CloseRange)))))

(fn GetHealthasRatio
  (return (/ (Variables|Default|GetHealth) (Variables|Default|GetMaxHealth))))