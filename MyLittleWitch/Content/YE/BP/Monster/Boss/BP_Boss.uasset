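; Dragon boss character that hunts the player and attacks based on distance until its health runs out.
; It chases via AIMoveTo while a looping timer picks random close-range montages or occasional far attacks: a fireball or staggered javelin volley.
; Toggleable fist and head colliders deal the attack's damage, with sphere traces for impact effects and a forward lunge event.
; Incoming damage triggers flinch reactions or a death sequence that destroys the actor.
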(event OnComponentBeginOverlap(Rt_Fist)
  (params (OverlappedComponent :type Primitive%20Component%20Object%20Reference) (OtherActor :type Actor%20Object%20Reference) (OtherComp :type Primitive%20Component%20Object%20Reference) (OtherBodyIndex :type Integer) (bFromSweep :type Boolean) (SweepResult :type Hit%20Result%20Structure%20%28by%20ref%29))
  ;[1 1 1] Fist Collision
  (if (== OtherActor (Game|GetPlayerCharacter 0))
    (CallFunction|DoDamage)
    ;;[1 1 1] Impulse
    (if (Variables|Default|GetIsAttacking)
      (Class|BPICharacter|GetHit(Message) OtherActor (Transformation|GetActorLocation)))))

(event OnComponentBeginOverlap(Lt_Fist)
  (params (OverlappedComponent :type Primitive%20Component%20Object%20Reference) (OtherActor :type Actor%20Object%20Reference) (OtherComp :type Primitive%20Component%20Object%20Reference) (OtherBodyIndex :type Integer) (bFromSweep :type Boolean) (SweepResult :type Hit%20Result%20Structure%20%28by%20ref%29))
  ;[1 1 1] Fist Collision
  (if (== OtherActor (Game|GetPlayerCharacter 0))
    (CallFunction|DoDamage)
    ;;[1 1 1] Impulse
    (if (Variables|Default|GetIsAttacking)
      (Class|BPICharacter|GetHit(Message) (stale OnComponentBeginOverlap(Rt_Fist) OtherActor) (Transformation|GetActorLocation)))))

(event OnComponentBeginOverlap(Head_Fist)
  (params (OverlappedComponent :type Primitive%20Component%20Object%20Reference) (OtherActor :type Actor%20Object%20Reference) (OtherComp :type Primitive%20Component%20Object%20Reference) (OtherBodyIndex :type Integer) (bFromSweep :type Boolean) (SweepResult :type Hit%20Result%20Structure%20%28by%20ref%29))
  ;[1 1 1] Fist Collision
  (if (== OtherActor (Game|GetPlayerCharacter 0))
    (CallFunction|DoDamage)
    ;;[1 1 1] Impulse
    (if (Variables|Default|GetIsAttacking)
      (Class|BPICharacter|GetHit(Message) (stale OnComponentBeginOverlap(Rt_Fist) OtherActor) (Transformation|GetActorLocation)))))

(event Custom|Launcher
  (bind _charactermovement (Variables|Character|GetCharacterMovement))
  ;[1 1 1] Launch to Character
  (Variables|/Script/Engine.CharacterMovementComponent|SetGroundFriction _charactermovement 0.0)
  (Character|LaunchCharacter (+ (* (Transformation|GetActorForwardVector) (Variables|Default|GetLaunchForce)) (* (Transformation|GetActorUpVector) (Variables|Default|GetJumpForce))) false false)
  (Utilities|FlowControl|RetriggerableDelay 25.0)
  (Variables|/Script/Engine.CharacterMovementComponent|SetGroundFriction _charactermovement 8.0))

(event Custom|Seek%20Player
  ;[1 1 1] Seek Player
  ;;[1 1 1] Flinch
  (if (Variables|Default|GetAlive)
    (if (not (Variables|Default|GetFlinch))
      (if (Variables|Default|GetIsAttacking)
        (Components|Movement|StopMovementImmediately (Variables|Character|GetCharacterMovement))
        (else
          ;;[1 1 1] Radius
          (AI|AIMoveTo self "0, 0, 0" (Game|GetPlayerCharacter 0) 2e+02 false
            (:then
              _)
            (:OnSuccess
              _)
            (:OnFail
              _))
          (Utilities|FlowControl|Delay 0.2)
          (CallFunction|SeekPlayer))))))

(event Custom|L%20Trace
  (bind _rt_fist (Variables|Default|GetRt_Fist))
  (bind _returnvalue (Transformation|GetWorldLocation _rt_fist))
  ;[1 1 1] ATK_EF
  (bind _outhit (Collision|SphereTraceForObjects _returnvalue (+ _returnvalue (* (Math|Vector|GetForwardVector (Transformation|GetWorldRotation _rt_fist)) 2e+02)) 64.0 (Utilities|Array|MakeArray "ObjectTypeQuery3") false 0 "None"))
  (if (== (.HitActor (Collision|BreakHitResult _outhit)) (Game|GetPlayerCharacter 0))
    (bind _returnvalue_2 (Effects|SpawnEmitteratLocation "/Game/YE/BP/Monster/Red/P_Buff_Red_AttackLava.P_Buff_Red_AttackLava" (.Location (Collision|BreakHitResult _outhit))))
    (Transformation|SetWorldScale3D _returnvalue_2 "2.000000,2.000000,2.000000")))

(event Custom|eCol%20Lt%20Fist
  ;[1 1 1] Fist Collision
  (Collision|SetCollisionEnabled (Variables|Default|GetLt_Fist) "QueryAndPhysics"))

(event Custom|H%20Trace
  (bind _rt_fist (Variables|Default|GetRt_Fist))
  (bind _returnvalue (Transformation|GetWorldLocation _rt_fist))
  ;[1 1 1] ATK_EF
  (bind _outhit (Collision|SphereTraceForObjects _returnvalue (+ _returnvalue (* (Math|Vector|GetForwardVector (Transformation|GetWorldRotation _rt_fist)) 3e+02)) 64.0 (Utilities|Array|MakeArray "ObjectTypeQuery3") false 0 "None"))
  (if (== (.HitActor (Collision|BreakHitResult _outhit)) (Game|GetPlayerCharacter 0))
    (bind _returnvalue_2 (Effects|SpawnEmitteratLocation "/Game/YE/BP/Monster/Red/P_Buff_Red_BigSmash_Impact.P_Buff_Red_BigSmash_Impact" (.Location (Collision|BreakHitResult _outhit))))
    (Transformation|SetWorldScale3D _returnvalue_2 "3.000000,3.000000,3.000000")))

(event Custom|Flame
  (bind _head_fist (Variables|Default|GetHead_Fist))
  (bind _returnvalue (Transformation|GetWorldLocation _head_fist))
  ;[1 1 1] Fireball
  (Game|SpawnActorfromClass "/Game/YE/BP/Monster/Boss/BP_Flame.BP_Flame_C" (Math|Transform|MakeTransform _returnvalue (Math|Rotator|FindLookatRotation _returnvalue (Transformation|GetActorLocation (Game|GetPlayerCharacter 0)))) "Undefined" 0 0))

(event Custom|Do%20Damage
  ;[1 1 1] Do Damage
  (Game|Damage|ApplyDamage (Game|GetPlayerCharacter 0) (Variables|Default|GetMaxDamage) 0 self))

(event Custom|dCol%20Head%20Fist
  ;[1 1 1] Fist Collision
  (Collision|SetCollisionEnabled (Variables|Default|GetHead_Fist) "NoCollision"))

(event Custom|eCol%20Head%20Fist
  ;[1 1 1] Fist Collision
  (Collision|SetCollisionEnabled (Variables|Default|GetHead_Fist) "QueryAndPhysics"))

(event Custom|Attack%20Jave
  ;[1 1 1] ATK Jave
  (Animation|PlayAnimMontage "/Game/YE/BP/Monster/Boss/Dragon_A_1_Fly_Ulti_Mon.Dragon_A_1_Fly_Ulti_Mon" 1.0 "None")
  (|Javelings
    (:execute2
      (Utilities|FlowControl|Delay 4.0)
      (Animation|PlayAnimMontage "/Game/YE/BP/Monster/Boss/Dragon_A_1_Fly_Ulti_Mon.Dragon_A_1_Fly_Ulti_Mon" 1.0 "None")
      (Utilities|FlowControl|Delay 4.0))))

(event Custom|Flying
  (Components|Animation|PlayAnimation (Variables|Character|GetMesh) "/Game/YE/BP/Monster/Boss/BS_Boss_Flying.BS_Boss_Flying" false))

(event Custom|Distance%20Player
  ;[1 1 1] Check Distance
  ;;[1 1 1] Flinch
  (if (Variables|Default|GetAlive)
    (if (not (Variables|Default|GetFlinch))
      ;;[1 1 1] How Often
      (Utilities|Time|SetTimerbyFunctionName 0 "Player Distance" 1.0 true))))

(event Custom|Close%20Range
  ;[1 1 1] Attack
  (Variables|Default|SetIsAttacking true)
  (switch int (Math|Random|RandomIntegerinRange 0 3)
    (:0
      (Variables|Default|SetATK_Montage "/Game/YE/BP/Monster/Boss/Animations/Dragon_A_1_Attack_1_Mon.Dragon_A_1_Attack_1_Mon")
      (Variables|Default|SetLaunchForce 3e+02)
      ;;[1 1 1] Damage
      (Variables|Default|SetMaxDamage 3e+01))
    (:1
      (Variables|Default|SetATK_Montage "/Game/YE/BP/Monster/Boss/Animations/Dragon_A_1_Attack_2_Mon.Dragon_A_1_Attack_2_Mon")
      (Variables|Default|SetLaunchForce 3e+02)
      (Variables|Default|SetMaxDamage 3e+01))
    (:2
      (Variables|Default|SetATK_Montage "/Game/YE/BP/Monster/Boss/Dragon_A_1_Breathe_Flame.Dragon_A_1_Breathe_Flame")
      (Variables|Default|SetLaunchForce 2e+02)
      (Variables|Default|SetMaxDamage 6e+01))
    (:3
      (Variables|Default|SetATK_Montage "/Game/YE/BP/Monster/Boss/Dragon_A_1_Breathe_Flame.Dragon_A_1_Breathe_Flame")
      (Variables|Default|SetLaunchForce 4e+02)
      (Variables|Default|SetMaxDamage 3e+01)))
  (bind _returnvalue (Animation|PlayAnimMontage (Variables|Default|GetATK_Montage) 1.0 "None"))
  (Utilities|FlowControl|Delay _returnvalue)
  ;;[1 1 1] Flinch
  (if (Variables|Default|GetAlive)
    (if (not (Variables|Default|GetFlinch))
      (Variables|Default|SetIsAttacking false)
      (CallFunction|SeekPlayer)
      ;[1 1 1] if Close  // Player Distance
      (if (not (>= (Variables|Default|GetDistance) 8.5e+02))
        (CallFunction|FacePlayer)))))

(event Custom|Far%20Range
  ;[1 1 1] Attack
  (Variables|Default|SetIsAttacking true)
  (switch int (Math|Random|RandomIntegerinRange 0 1)
    (:0
      (CallFunction|Flame)
      (Variables|Default|SetATK_Montage 0)
      (Variables|Default|SetMaxDamage 6e+01))
    (:1
      (CallFunction|AttackJave)
      (Variables|Default|SetMaxDamage 3e+01)))
  (bind _returnvalue (Animation|PlayAnimMontage (Variables|Default|GetATK_Montage) 1.0 "None"))
  (Utilities|FlowControl|Delay _returnvalue)
  ;;[1 1 1] Flinch
  (if (Variables|Default|GetAlive)
    (if (not (Variables|Default|GetFlinch))
      (Variables|Default|SetIsAttacking false)
      (CallFunction|SeekPlayer)
      ;[1 1 1] if Close  // Player Distance
      (if (not (>= (Variables|Default|GetDistance) 8.5e+02))
        (CallFunction|FacePlayer)))))

(event Custom|Face%20Player
  ;[1 1 1] Face to Player
  (Transformation|SetActorRotation (Math|Rotator|FindLookatRotation (Transformation|GetActorLocation) (Transformation|GetActorLocation (Game|GetPlayerCharacter 0)))))

(event Custom|dCol%20Rt%20Fist
  ;[1 1 1] Fist Collision
  (Collision|SetCollisionEnabled (Variables|Default|GetRt_Fist) "NoCollision"))

(event Custom|dCol%20Lt%20Fist
  ;[1 1 1] Fist Collision
  (Collision|SetCollisionEnabled (Variables|Default|GetLt_Fist) "NoCollision"))

(event Custom|R%20Trace
  (bind _rt_fist (Variables|Default|GetRt_Fist))
  (bind _returnvalue (Transformation|GetWorldLocation _rt_fist))
  ;[1 1 1] ATK_EF
  (bind _outhit (Collision|SphereTraceForObjects _returnvalue (+ _returnvalue (* (Math|Vector|GetForwardVector (Transformation|GetWorldRotation _rt_fist)) 2e+02)) 64.0 (Utilities|Array|MakeArray "ObjectTypeQuery3") false 0 "None"))
  (if (== (.HitActor (Collision|BreakHitResult _outhit)) (Game|GetPlayerCharacter 0))
    (bind _returnvalue_2 (Effects|SpawnEmitteratLocation "/Game/YE/BP/Monster/Red/P_Buff_Red_AttackLava.P_Buff_Red_AttackLava" (.Location (Collision|BreakHitResult _outhit))))
    (Transformation|SetWorldScale3D _returnvalue_2 "2.000000,2.000000,2.000000")))

(event Custom|eCol%20Rt%20Fist
  ;[1 1 1] Fist Collision
  (Collision|SetCollisionEnabled (Variables|Default|GetRt_Fist) "QueryAndPhysics"))

(event EventBeginPlay
  ;[1 1 1] Base
  (Variables|Default|SetAlive true)
  (Utilities|FlowControl|Delay 0.2)
  (CallFunction|SeekPlayer)
  (CallFunction|DistancePlayer)
  (Variables|Default|SetHealth 1e+02))

(event Game|Damage|EventAnyDamage
  (params (Damage :type Float%20%28single-precision%29) (DamageType :type Damage%20Type%20Object%20Reference) (InstigatedBy :type Controller%20Object%20Reference) (DamageCauser :type Actor%20Object%20Reference))
  ;[1 1 1] Get  Damage
  (if (!= DamageCauser self)
    (Variables|Default|SetDamage Damage)
    (bind _output_get (Variables|Default|SetHealth (- (Variables|Default|GetHealth) Damage)))
    (if (<= _output_get 0.0)
      (Animation|PlayAnimMontage "/Game/YE/BP/Monster/Black/Knock_back_Mon.Knock_back_Mon" 0.25 "None" :!label _label)
      (Utilities|FlowControl|Delay 0.2)
      (Effects|SpawnEmitterAttached "/Game/YE/BP/Monster/Red/P_CarriedBuff_GroundPickup_Red.P_CarriedBuff_GroundPickup_Red" (Variables|Character|GetMesh) "None" "0, 0, 0" "0, 0, 0" "3.000000,3.000000,3.000000")
      (Utilities|FlowControl|Delay 0.3)
      (Variables|Default|SetAlive false)
      (Utilities|FlowControl|Delay 0.2)
      (Actor|DestroyActor)
      (elif (>= (Variables|Default|GetDamage) 5.0)
        (Variables|Default|SetFlinch true)
        (switch int (Math|Random|RandomIntegerinRange 0 2)
          (:0
            (Variables|Default|SetATK_Montage "/Game/YE/BP/Monster/Black/Hitreact_Front_Mon.Hitreact_Front_Mon"))
          (:1
            (Variables|Default|SetATK_Montage "/Game/YE/BP/Monster/Black/Hitreact_Left_Mon.Hitreact_Left_Mon"))
          (:2
            (Variables|Default|SetATK_Montage "/Game/YE/BP/Monster/Black/Hitreact_Right_Mon.Hitreact_Right_Mon")))
        (bind _returnvalue (Animation|PlayAnimMontage (Variables|Default|GetATK_Montage) 1.0 "None"))
        (Utilities|FlowControl|Delay _returnvalue)
        (Variables|Default|SetFlinch false)
        (if (<= (Variables|Default|GetHealth) 0.0)
          (goto _label))))))

(event EventDotDamage
  (params (Damage :type Float%20%28single-precision%29))
  ;[1 1 1] Dot damage 피격
  (if (not (Variables|Default|GetDot))
    (Variables|Default|SetDot true)
    (Variables|Default|SetHealth (- (Variables|Default|GetHealth) Damage))
    (Animation|PlayAnimMontage self 0 1.0 "None")
    (Utilities|FlowControl|Delay 0.1)
    (Variables|Default|SetDot false)))

(fn ConstructionScript)

(fn PlayerDistance
  ;[1 1 1] Distance
  (if (Variables|Default|GetAlive)
    (if (not (and (Variables|Default|GetIsAttacking) (Variables|Default|GetFlinch)))
      ;;[1 1 1] Detect
      (bind _output_get (Variables|Default|SetDistance (Math|Vector|VectorLength (- (Transformation|GetActorLocation) (Transformation|GetActorLocation (Game|GetPlayerCharacter 0))))))
      ;;[1 1 1] Far
      (if (>= _output_get 8.5e+02)
        (if (== (Math|Random|RandomIntegerinRange 0 4) 0)
          (CallFunction|FarRange)
          (else
            (CallFunction|SeekPlayer)))
        (else
          (CallFunction|CloseRange))))))