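; Boss skill Blueprint that, on BeginPlay, plays a montage and launches a volley of javelins.
; The Javelings macro spawns three BPA_Javelings in a row above the boss, each with its own offset and staggered charge delay.
; A delayed repeat follows the macro, but its output is never reached, so the volley fires once.
; The Attack slan projectile macro is left unconnected.
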(event Custom|Attack%20Sword
  (Animation|PlayAnimMontage "/Game/YE/BP/Monster/Boss/Skills/Idle_Variant_01_Mon.Idle_Variant_01_Mon" 1.0 "None")
  (|Javelings
    (:OutputPin
      (Utilities|FlowControl|Delay 4.0)
      (Animation|PlayAnimMontage "/Game/YE/BP/Monster/Boss/Skills/Idle_Variant_01_Mon.Idle_Variant_01_Mon" 1.0 "None")
      (Utilities|FlowControl|Delay 4.0)
      ;[1 1 1] Want Repeat
      (CallFunction|AttackSword))))

(event EventBeginPlay
  (CallFunction|AttackSword))

(event Collision|EventActorBeginOverlap
  (params (OtherActor :type Actor%20Object%20Reference)))

(event EventTick
  (params (DeltaSeconds :type Float%20%28single-precision%29)))

(fn ConstructionScript)