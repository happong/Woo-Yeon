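; Mid-boss enemy that chases the player, makes melee attacks, and on death increments BP_Portal1's death count and calls OpenPortal.
; A recursive AIMoveTo loop seeks, while a looping distance timer triggers random punch or smash montages.
; Toggleable fist collisions deal damage, sphere traces spawn hit effects, and Launcher lunges the boss forward.
; Damage drives flinch reactions and death; the HP widget receives the boss as health interface; Phase 2 is unfinished.
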(event OnComponentBeginOverlap(Rt_Fist)
  (params (OverlappedComponent :type Primitive%20Component%20Object%20Reference) (OtherActor :type Actor%20Object%20Reference) (OtherComp :type Primitive%20Component%20Object%20Reference) (OtherBodyIndex :type Integer) (bFromSweep :type Boolean) (SweepResult :type Hit%20Result%20Structure%20%28by%20ref%29))
  ;[1 1 1] Fist Collision
  (if (== OtherActor (Game|GetPlayerCharacter 0))
    (CallFunction|DoDamage)
    ;;[1 1 1] Impulse
    (if (Variables|Default|GetIsAttacking)
      (Class|BPICharacter|GetHit(Message) OtherActor (Transformation|GetActorLocation)))))

(event OnComponentBeginOverlap(Lt_Fist)
  (params (OverlappedComponent :type Primitive%20Component%20Object%20Reference) (OtherActor :type Actor%20Object%20Reference) (OtherComp :type Primitive%20Component%20Object%20Reference) (OtherBodyIndex :type Integer) (bFromSweep :type Boolean) (SweepResult :type Hit%20Result%20Structure%20%28by%20ref%29))
  ;[1 1 1] Fist Collision
  (if (== OtherActor (Game|GetPlayerCharacter 0))
    (CallFunction|DoDamage)
    ;;[1 1 1] Impulse
    (if (Variables|Default|GetIsAttacking)
      (Class|BPICharacter|GetHit(Message) (stale OnComponentBeginOverlap(Rt_Fist) OtherActor) (Transformation|GetActorLocation)))))

(event Custom|Launcher
  (bind _charactermovement (Variables|Character|GetCharacterMovement))
  ;[1 1 1] Launch to Character
  (Variables|/Script/Engine.CharacterMovementComponent|SetGroundFriction _charactermovement 0.0)
  (Character|LaunchCharacter (+ (* (Transformation|GetActorForwardVector) (Variables|Default|GetLaunchForce)) (* (Transformation|GetActorUpVector) (Variables|Default|GetJumpForce))) false false)
  (Utilities|FlowControl|RetriggerableDelay 25.0)
  (Variables|/Script/Engine.CharacterMovementComponent|SetGroundFriction _charactermovement 8.0))

(event Custom|Seek%20Player
  ;[1 1 1] Seek Player
  ;;[1 1 1] Flinch
  (if (Variables|Default|GetAlive)
    (if (not (Variables|Default|GetFlinch))
      (if (Variables|Default|GetIsAttacking)
        (Components|Movement|StopMovementImmediately (Variables|Character|GetCharacterMovement))
        (else
          ;;[1 1 1] Radius
          (AI|AIMoveTo self "0, 0, 0" (Game|GetPlayerCharacter 0) 2e+02 false
            (:then
              _)
            (:OnSuccess
              _)
            (:OnFail
              _))
          (Utilities|FlowControl|Delay 1.0)
          (CallFunction|SeekPlayer))))))

(event Custom|L%20Trace
  (bind _lt_fist (Variables|Default|GetLt_Fist))
  (bind _returnvalue (Transformation|GetWorldLocation _lt_fist))
  ;[1 1 1] ATK_EF
  (bind _outhit (Collision|SphereTraceForObjects _returnvalue (+ _returnvalue (* (Math|Vector|GetForwardVector (Transformation|GetWorldRotation _lt_fist)) 2e+02)) 64.0 (Utilities|Array|MakeArray "ObjectTypeQuery3") false 0 "None"))
  (if (== (.HitActor (Collision|BreakHitResult _outhit)) (Game|GetPlayerCharacter 0))
    (bind _returnvalue_2 (Effects|SpawnEmitteratLocation "/Game/YE/BP/Monster/MidBoss/P_Revenant_FrostKing_Mark_End.P_Revenant_FrostKing_Mark_End" (.Location (Collision|BreakHitResult _outhit))))
    (Transformation|SetWorldScale3D _returnvalue_2 "3.000000,3.000000,3.000000")))

(event Custom|eCol%20Lt%20Fist
  ;[1 1 1] Fist Collision
  (Collision|SetCollisionEnabled (Variables|Default|GetLt_Fist) "QueryAndPhysics"))

(event Custom|Smash%20Trace
  (bind _rt_fist (Variables|Default|GetRt_Fist))
  (bind _returnvalue (Transformation|GetWorldLocation _rt_fist))
  ;[1 1 1] ATK_EF
  (bind _outhit (Collision|SphereTraceForObjects _returnvalue (+ _returnvalue (* (Math|Vector|GetForwardVector (Transformation|GetWorldRotation _rt_fist)) 3e+02)) 64.0 (Utilities|Array|MakeArray "ObjectTypeQuery3") false 0 "None"))
  (if (== (.HitActor (Collision|BreakHitResult _outhit)) (Game|GetPlayerCharacter 0))
    (bind _returnvalue_2 (Effects|SpawnEmitteratLocation "/Game/YE/BP/Monster/MidBoss/P_Rampage_Ice_Rock_HitWorld.P_Rampage_Ice_Rock_HitWorld" (.Location (Collision|BreakHitResult _outhit))))
    (Transformation|SetWorldScale3D _returnvalue_2 "2.000000,2.000000,2.000000")))

(event Custom|Do%20Damage
  ;[1 1 1] Do Damage
  (Game|Damage|ApplyDamage (Game|GetPlayerCharacter 0) (Variables|Default|GetMaxDamage) 0 self))

(event Custom|Change%20Phase2
  ;[1 1 1] Attack
  ;;[1 1 1] X
)

(event Custom|Distance%20Player
  ;[1 1 1] Check Distance
  ;;[1 1 1] Flinch
  (if (Variables|Default|GetAlive)
    (if (not (Variables|Default|GetFlinch))
      ;;[1 1 1] How Often
      (Utilities|Time|SetTimerbyFunctionName 0 "Player Distance" 1.0 true))))

(event Custom|Close%20Range
  ;[1 1 1] Attack
  (Variables|Default|SetIsAttacking true)
  (Utilities|FlowControl|Delay 0.5)
  (switch int (Math|Random|RandomIntegerinRange 0 4)
    (:0
      (Variables|Default|SetATK_Montage "/Game/YE/BP/Monster/MidBoss/Animations/Attack_Melee_A_Mon.Attack_Melee_A_Mon")
      (Variables|Default|SetLaunchForce 3e+02)
      ;;[1 1 1] Damage
      (Variables|Default|SetMaxDamage 1e+01)
      (bind _returnvalue (Animation|PlayAnimMontage (Variables|Default|GetATK_Montage) 0.8 "None" :!label _label))
      (Utilities|FlowControl|Delay _returnvalue))
    (:1
      (Variables|Default|SetATK_Montage "/Game/YE/BP/Monster/MidBoss/Animations/Attack_Melee_B_Mon.Attack_Melee_B_Mon")
      (Variables|Default|SetLaunchForce 3e+02)
      (Variables|Default|SetMaxDamage 1e+01)
      (goto _label))
    (:2
      (Variables|Default|SetATK_Montage "/Game/YE/BP/Monster/MidBoss/Animations/Attack_Melee_C_Mon.Attack_Melee_C_Mon")
      (Variables|Default|SetLaunchForce 2e+02)
      (Variables|Default|SetMaxDamage 15.0)
      (goto _label))
    (:3
      (Variables|Default|SetATK_Montage "/Game/YE/BP/Monster/MidBoss/Ability_GroundSmash_End_Mon.Ability_GroundSmash_End_Mon")
      (Variables|Default|SetMaxDamage 1e+02)
      (bind _returnvalue_2 (Animation|PlayAnimMontage (Variables|Default|GetATK_Montage) 0.6 "None" :!label _label_2))
      (Utilities|FlowControl|Delay _returnvalue_2))
    (:4
      (Variables|Default|SetATK_Montage "/Game/YE/BP/Monster/MidBoss/Ability_RMB_Smash_Mon.Ability_RMB_Smash_Mon")
      (Variables|Default|SetMaxDamage 1e+02)
      (goto _label_2)))
  ;;[1 1 1] Flinch
  (if (Variables|Default|GetAlive)
    (if (not (Variables|Default|GetFlinch))
      (Variables|Default|SetIsAttacking false)
      (CallFunction|SeekPlayer)
      ;[1 1 1] if Close  // Player Distance
      (if (not (>= (Variables|Default|GetDistance) 8.5e+02))
        (CallFunction|FacePlayer)))))

(event Custom|Face%20Player
  ;[1 1 1] Face to Player
  (Transformation|SetActorRotation (Math|Rotator|FindLookatRotation (Transformation|GetActorLocation) (Transformation|GetActorLocation (Game|GetPlayerCharacter 0)))))

(event Custom|dCol%20Rt%20Fist
  ;[1 1 1] Fist Collision
  (Collision|SetCollisionEnabled (Variables|Default|GetRt_Fist) "NoCollision"))

(event Custom|dCol%20Lt%20Fist
  ;[1 1 1] Fist Collision
  (Collision|SetCollisionEnabled (Variables|Default|GetLt_Fist) "NoCollision"))

(event Custom|R%20Trace
  (bind _rt_fist (Variables|Default|GetRt_Fist))
  (bind _returnvalue (Transformation|GetWorldLocation _rt_fist))
  ;[1 1 1] ATK_EF
  (bind _outhit (Collision|SphereTraceForObjects _returnvalue (+ _returnvalue (* (Math|Vector|GetForwardVector (Transformation|GetWorldRotation _rt_fist)) 2e+02)) 64.0 (Utilities|Array|MakeArray "ObjectTypeQuery3") false 0 "None"))
  (if (== (.HitActor (Collision|BreakHitResult _outhit)) (Game|GetPlayerCharacter 0))
    (bind _returnvalue_2 (Effects|SpawnEmitteratLocation "/Game/YE/BP/Monster/MidBoss/P_Revenant_FrostKing_Mark_End.P_Revenant_FrostKing_Mark_End" (.Location (Collision|BreakHitResult _outhit))))
    (Transformation|SetWorldScale3D _returnvalue_2 "3.000000,3.000000,3.000000")))

(event Custom|eCol%20Rt%20Fist
  ;[1 1 1] Fist Collision
  (Collision|SetCollisionEnabled (Variables|Default|GetRt_Fist) "QueryAndPhysics"))

(event EventBeginPlay
  ;[1 1 1] Base
  (Variables|Default|SetHealth (Variables|Default|GetMaxHealth))
  (bind _aswb_mid_boss_hp (Utilities|Casting|CastToWB_MidBossHP (UserInterface|GetUserWidgetObject (Variables|Default|GetHP%20Bar))))
  (Variables|/Game/YE/WB/WB_MidBossHP.WB_MidBossHP_C|SetHealthInterface _aswb_mid_boss_hp self)
  (Variables|Default|SetAlive true)
  (Variables|Default|SetPhase2 false)
  (Utilities|FlowControl|Delay 0.2)
  (CallFunction|SeekPlayer)
  (CallFunction|DistancePlayer)
  (bind _returnvalue (Actor|GetActorOfClass "/Game/Developers/haeun/Collections/blueprint/BP_Portal1.BP_Portal1_C"))
  (Variables|Default|SetPortalVar _returnvalue))

(event Game|Damage|EventAnyDamage
  (params (Damage :type Float%20%28single-precision%29) (DamageType :type Damage%20Type%20Object%20Reference) (InstigatedBy :type Controller%20Object%20Reference) (DamageCauser :type Actor%20Object%20Reference))
  (bind _portalvar (Variables|Default|GetPortalVar))
  ;[1 1 1] Get  Damage
  (if (!= DamageCauser self)
    (Variables|Default|SetDamage Damage)
    (bind _output_get (Variables|Default|SetHealth (- (Variables|Default|GetHealth) Damage)))
    ;;[1 1 1] Portal
    (if (<= _output_get 0.0)
      (Variables|/Game/Developers/haeun/Collections/blueprint/BP_Portal1.BP_Portal1_C|SetdeathCount _portalvar (+ (Variables|/Game/Developers/haeun/Collections/blueprint/BP_Portal1.BP_Portal1_C|GetdeathCount _portalvar) 1.0))
      (Default|OpenPortal _portalvar)
      (Utilities|FlowControl|Delay 0.2)
      (Animation|PlayAnimMontage "/Game/YE/BP/Monster/MidBoss/Animations/Death_A_Mon.Death_A_Mon" 0.5 "None" :!label _label)
      (Effects|SpawnEmitterAttached "/Game/YE/BP/Monster/MidBoss/P_Rampage_Ice_Enrage_End.P_Rampage_Ice_Enrage_End" (Variables|Character|GetMesh) "None" "0, 0, 0" "0, 0, 0" "3.000000,3.000000,3.000000")
      (Utilities|FlowControl|Delay 0.3)
      (Variables|Default|SetAlive false)
      (Utilities|FlowControl|Delay 0.2)
      (Actor|DestroyActor)
      (elif (>= (Variables|Default|GetDamage) 5.0)
        (Variables|Default|SetFlinch true)
        (switch int (Math|Random|RandomIntegerinRange 0 2)
          (:0
            (Variables|Default|SetATK_Montage "/Game/YE/BP/Monster/MidBoss/Animations/HitReact_Front_Mon.HitReact_Front_Mon"))
          (:1
            (Variables|Default|SetATK_Montage "/Game/YE/BP/Monster/MidBoss/Animations/HitReact_Right_Mon.HitReact_Right_Mon"))
          (:2
            (Variables|Default|SetATK_Montage "/Game/YE/BP/Monster/MidBoss/Animations/HitReact_Left_Mon.HitReact_Left_Mon")))
        (bind _returnvalue (Animation|PlayAnimMontage (Variables|Default|GetATK_Montage) 1.0 "None"))
        (Utilities|FlowControl|Delay _returnvalue)
        (Variables|Default|SetFlinch false)
        (if (<= (Variables|Default|GetHealth) 0.0)
          (goto _label))))))

(event EventDotDamage
  (params (Damage :type Float%20%28single-precision%29))
  ;[1 1 1] Dot damage 피격
  (if (not (Variables|Default|GetDot))
    (Variables|Default|SetDot true)
    (Variables|Default|SetHealth (- (Variables|Default|GetHealth) Damage))
    (Animation|PlayAnimMontage self 0 1.0 "None")
    (Utilities|FlowControl|Delay 0.1)
    (Variables|Default|SetDot false)))

(fn ConstructionScript)

(fn PlayerDistance
  ;[1 1 1] Distance
  (if (Variables|Default|GetAlive)
    (if (not (and (Variables|Default|GetIsAttacking) (Variables|Default|GetFlinch)))
      ;;[1 1 1] Detect
      (bind _output_get (Variables|Default|SetDistance (Math|Vector|VectorLength (- (Transformation|GetActorLocation) (Transformation|GetActorLocation (Game|GetPlayerCharacter 0))))))
      ;;[1 1 1] Far
      (if (not (> _output_get 1e+03))
        (if (>= _output_get 7.5e+02)
          (if (== (Math|Random|RandomIntegerinRange 0 4) 0)
            (CallFunction|CloseRange)
            (else
              (CallFunction|SeekPlayer)))
          (else
            (CallFunction|CloseRange)))))))

(fn GetHealthasRatio
  (return (/ (Variables|Default|GetHealth) (Variables|Default|GetMaxHealth))))