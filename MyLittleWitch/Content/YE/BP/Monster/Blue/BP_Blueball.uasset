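; BP_Blueball is a monster attack orb that damages the player on overlap and destroys itself.
; It enables sphere collision shortly after spawning and expires on a timer if it hits nothing.
; Overlaps send a hit message with the orb's location to the other actor.
; Contact with SerathPlayerCharacter applies MaxDamage, spawns a blue particle effect and removes the orb.
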(event OnComponentBeginOverlap(Sphere)
  (params (OverlappedComponent :type Primitive%20Component%20Object%20Reference) (OtherActor :type Actor%20Object%20Reference) (OtherComp :type Primitive%20Component%20Object%20Reference) (OtherBodyIndex :type Integer) (bFromSweep :type Boolean) (SweepResult :type Hit%20Result%20Structure%20%28by%20ref%29))
  ;[1 1 1] Base
  ;;[1 1 1] Impulse
  (if (Variables|Default|Getattacking)
    (Class|BPICharacter|GetHit(Message) OtherActor (Transformation|GetActorLocation))
    (if (== (Utilities|GetClass OtherActor) "/Game/YE/SerathPlayerCharacter.SerathPlayerCharacter_C")
      (Utilities|Casting|CastToSerathPlayerCharacter (Game|GetPlayerCharacter 0))
      (CallFunction|DoDamage)
      (Effects|SpawnEmitteratLocation "/Game/YE/BP/Monster/Blue/P_CarriedBuff_GroundPickup_Mid_Blue.P_CarriedBuff_GroundPickup_Mid_Blue" (Transformation|GetWorldLocation (Variables|Default|GetSphere)))
      (Utilities|FlowControl|Delay 0.05)
      (Actor|DestroyActor))))

(event Custom|Do%20Damage
  ;[1 1 1] Do Damage
  (Game|Damage|ApplyDamage (Game|GetPlayerCharacter 0) (Variables|Default|GetMax%20Damage) 0 self))

(event EventBeginPlay
  (Variables|Default|Setattacking true)
  (Utilities|FlowControl|Delay 0.2)
  (Collision|SetCollisionEnabled (Variables|Default|GetSphere) "QueryAndPhysics")
  (Utilities|FlowControl|Delay 6.0)
  (Actor|DestroyActor))

(fn ConstructionScript)