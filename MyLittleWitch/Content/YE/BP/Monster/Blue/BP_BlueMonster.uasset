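; Blue monster enemy that chases the player, attacks in melee or at range, and shows health through an HP widget.
; A looping distance timer picks a fist attack up close, or at range randomly either keeps chasing via AIMoveTo or plays a fire montage.
; Separate events toggle fist collision, trace hit effects and launch Blueball or Iceball projectiles at the player.
; Heavier hits trigger random flinch montages, and zero health plays death effects before destroying the actor.
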(event OnComponentBeginOverlap(Body_Fist)
  (params (OverlappedComponent :type Primitive%20Component%20Object%20Reference) (OtherActor :type Actor%20Object%20Reference) (OtherComp :type Primitive%20Component%20Object%20Reference) (OtherBodyIndex :type Integer) (bFromSweep :type Boolean) (SweepResult :type Hit%20Result%20Structure%20%28by%20ref%29))
  ;[1 1 1] Fist Collision
  (if (== OtherActor (Game|GetPlayerCharacter 0))
    (CallFunction|DoDamage)
    ;;[1 1 1] Impulse
    (if (Variables|Default|GetIsAttacking)
      (Class|BPICharacter|GetHit(Message) OtherActor (Transformation|GetActorLocation)))))

(event Custom|Iceball
  (bind _head (Variables|Default|GetHead))
  (bind _returnvalue (Transformation|GetWorldLocation _head))
  ;[1 1 1] Iceball
  (Game|SpawnActorfromClass "/Game/YE/BP/Monster/Blue/BP_Iceball.BP_Iceball_C" (Math|Transform|MakeTransform _returnvalue (Math|Rotator|FindLookatRotation _returnvalue (Transformation|GetActorLocation (Game|GetPlayerCharacter 0)))) "Undefined" 0 0))

(event Custom|Seek%20Player
  ;[1 1 1] Seek Player
  ;;[1 1 1] Flinch
  (if (Variables|Default|GetAlive)
    (if (not (Variables|Default|GetFlinch))
      (if (Variables|Default|GetIsAttacking)
        (Components|Movement|StopMovementImmediately (Variables|Character|GetCharacterMovement))
        (else
          ;;[1 1 1] Radius
          (AI|AIMoveTo self "0, 0, 0" (Game|GetPlayerCharacter 0) 2e+02 false
            (:then
              _)
            (:OnSuccess
              _)
            (:OnFail
              _))
          (Utilities|FlowControl|Delay 0.2)
          (CallFunction|SeekPlayer))))))

(event Custom|Blueball
  (bind _head (Variables|Default|GetHead))
  (bind _returnvalue (Transformation|GetWorldLocation _head))
  ;[1 1 1] Blueball
  (Game|SpawnActorfromClass "/Game/YE/BP/Monster/Blue/BP_Blueball.BP_Blueball_C" (Math|Transform|MakeTransform _returnvalue (Math|Rotator|FindLookatRotation _returnvalue (Transformation|GetActorLocation (Game|GetPlayerCharacter 0)))) "Undefined" 0 0))

(event Custom|Do%20Damage
  ;[1 1 1] Do Damage
  (Game|Damage|ApplyDamage (Game|GetPlayerCharacter 0) (Variables|Default|GetMaxDamage) 0 self))

(event Custom|Distance%20Player
  ;[1 1 1] Check Distance
  ;;[1 1 1] Flinch
  (if (Variables|Default|GetAlive)
    (if (not (Variables|Default|GetFlinch))
      ;;[1 1 1] How Often
      (Utilities|Time|SetTimerbyFunctionName 0 "Player Distance" 1.0 true))))

(event Custom|Close%20Range
  ;[1 1 1] Attack
  (Variables|Default|SetIsAttacking true)
  (switch int 0
    (:0
      (Variables|Default|SetATK_Montage "/Game/YE/BP/Monster/Blue/Animations/Attack_Mon.Attack_Mon")
      ;;[1 1 1] Damage
      (Variables|Default|SetMaxDamage 1e+01)
      (bind _returnvalue (Animation|PlayAnimMontage (Variables|Default|GetATK_Montage) 1.0 "None"))
      (Utilities|FlowControl|Delay _returnvalue)
      ;;[1 1 1] Flinch
      (if (Variables|Default|GetAlive)
        (if (not (Variables|Default|GetFlinch))
          (Variables|Default|SetIsAttacking false)
          (CallFunction|SeekPlayer)
          ;[1 1 1] if Close  // Player Distance
          (if (not (>= (Variables|Default|GetDistance) 8.5e+02))
            (CallFunction|FacePlayer)))))))

(event Custom|Far%20Range
  ;[1 1 1] Attack
  (Variables|Default|SetIsAttacking true)
  (switch int (Math|Random|RandomIntegerinRange 0 1)
    (:0
      (Variables|Default|SetATK_Montage "/Game/YE/BP/Monster/Blue/Animations/Fire_Mon.Fire_Mon")
      ;;[1 1 1] Damage
      (Variables|Default|SetMaxDamage 1e+01))
    (:1
      (Variables|Default|SetATK_Montage "/Game/YE/BP/Monster/Blue/Animations/Fire_B_Mon.Fire_B_Mon")
      (Variables|Default|SetMaxDamage 1e+01)))
  (bind _returnvalue (Animation|PlayAnimMontage (Variables|Default|GetATK_Montage) 1.0 "None"))
  (Utilities|FlowControl|Delay _returnvalue)
  ;;[1 1 1] Flinch
  (if (Variables|Default|GetAlive)
    (if (not (Variables|Default|GetFlinch))
      (Variables|Default|SetIsAttacking false)
      (CallFunction|SeekPlayer)
      ;[1 1 1] if Close  // Player Distance
      (if (not (>= (Variables|Default|GetDistance) 8.5e+02))
        (CallFunction|FacePlayer)))))

(event Custom|Face%20Player
  ;[1 1 1] Face to Player
  (Transformation|SetActorRotation (Math|Rotator|FindLookatRotation (Transformation|GetActorLocation) (Transformation|GetActorLocation (Game|GetPlayerCharacter 0)))))

(event Custom|dCol%20B%20Fist
  ;[1 1 1] Fist Collision
  (Collision|SetCollisionEnabled (Variables|Default|GetBody_Fist) "NoCollision"))

(event Custom|ATK%20Trace
  (bind _body_fist (Variables|Default|GetBody_Fist))
  (bind _returnvalue (Transformation|GetWorldLocation _body_fist))
  ;[1 1 1] ATK_EF
  (bind _outhit (Collision|SphereTraceForObjects _returnvalue (+ _returnvalue (* (Math|Vector|GetForwardVector (Transformation|GetWorldRotation _body_fist)) 2e+02)) 64.0 (Utilities|Array|MakeArray "ObjectTypeQuery3") false 0 "None"))
  (if (== (.HitActor (Collision|BreakHitResult _outhit)) (Game|GetPlayerCharacter 0))
    (bind _returnvalue_2 (Effects|SpawnEmitteratLocation "/Game/YE/BP/Monster/Blue/P_CarriedBuff_GroundPickup_Blue.P_CarriedBuff_GroundPickup_Blue" (.Location (Collision|BreakHitResult _outhit))))
    (Transformation|SetWorldScale3D _returnvalue_2 "2.000000,2.000000,2.000000")))

(event Custom|eCol%20B%20Fist
  ;[1 1 1] Fist Collision
  (Collision|SetCollisionEnabled (Variables|Default|GetBody_Fist) "QueryAndPhysics"))

(event EventBeginPlay
  ;[1 1 1] Base
  (Variables|Default|SetHealth (Variables|Default|GetMaxHealth))
  (bind _aswb_blue_monster_hp (Utilities|Casting|CastToWB_BlueMonsterHP (UserInterface|GetUserWidgetObject (Variables|Default|GetHP%20Bar))))
  (Variables|/Game/YE/WB/WB_BlueMonsterHP.WB_BlueMonsterHP_C|SetHealthInterface _aswb_blue_monster_hp self)
  (Variables|Default|SetAlive true)
  (Utilities|FlowControl|Delay 0.2)
  (CallFunction|SeekPlayer)
  (CallFunction|DistancePlayer))

(event Game|Damage|EventAnyDamage
  (params (Damage :type Float%20%28single-precision%29) (DamageType :type Damage%20Type%20Object%20Reference) (InstigatedBy :type Controller%20Object%20Reference) (DamageCauser :type Actor%20Object%20Reference))
  ;[1 1 1] Get  Damage
  (if (!= DamageCauser self)
    (Variables|Default|SetDamage Damage)
    (bind _output_get (Variables|Default|SetHealth (- (Variables|Default|GetHealth) Damage)))
    (if (<= _output_get 0.0)
      (Animation|PlayAnimMontage "/Game/YE/BP/Monster/Blue/Animations/Death_Fwd_Mon.Death_Fwd_Mon" 1.0 "None" :!label _label)
      (Utilities|FlowControl|Delay 1.0)
      (Effects|SpawnEmitterAttached "/Game/YE/BP/Monster/Blue/P_Blue_Buff_Babies_Spew.P_Blue_Buff_Babies_Spew" (Variables|Character|GetMesh) "None" "0, 0, 0" "0, 0, 0" "3.000000,3.000000,3.000000")
      (Utilities|FlowControl|Delay 0.3)
      (Variables|Default|SetAlive false)
      (Utilities|FlowControl|Delay 0.2)
      (Actor|DestroyActor)
      (elif (>= (Variables|Default|GetDamage) 5.0)
        (Variables|Default|SetFlinch true)
        (switch int (Math|Random|RandomIntegerinRange 0 3)
          (:0
            (Variables|Default|SetATK_Montage "/Game/YE/BP/Monster/Blue/Animations/Hitreat_Fwd_Mon.Hitreat_Fwd_Mon"))
          (:1
            (Variables|Default|SetATK_Montage "/Game/YE/BP/Monster/Blue/Animations/Hitreat_Left_Mon.Hitreat_Left_Mon"))
          (:2
            (Variables|Default|SetATK_Montage "/Game/YE/BP/Monster/Blue/Animations/Hitreat_Right_Mon.Hitreat_Right_Mon"))
          (:3
            (Variables|Default|SetATK_Montage "/Game/YE/BP/Monster/Blue/Animations/KnockBack_Bwd_Mon.KnockBack_Bwd_Mon")))
        (bind _returnvalue (Animation|PlayAnimMontage (Variables|Default|GetATK_Montage) 1.0 "None"))
        (Utilities|FlowControl|Delay _returnvalue)
        (Variables|Default|SetFlinch false)
        (if (<= (Variables|Default|GetHealth) 0.0)
          (goto _label))))))

(event EventDotDamage
  (params (Damage :type Float%20%28single-precision%29))
  ;[1 1 1] Dot Damage 피격
  (if (not (Variables|Default|GetDot))
    (Variables|Default|SetDot true)
    (Variables|Default|SetHealth (- (Variables|Default|GetHealth) 1.0))
    (Animation|PlayAnimMontage self 0 1.0 "None")
    (Utilities|FlowControl|Delay 0.1)
    (Variables|Default|SetDot false)))

(fn ConstructionScript)

(fn PlayerDistance
  ;[1 1 1] Distance
  (if (Variables|Default|GetAlive)
    (if (not (and (Variables|Default|GetIsAttacking) (Variables|Default|GetFlinch)))
      ;;[1 1 1] Detect
      (bind _output_get (Variables|Default|SetDistance (Math|Vector|VectorLength (- (Transformation|GetActorLocation) (Transformation|GetActorLocation (Game|GetPlayerCharacter 0))))))
      ;;[1 1 1] Far
      (if (>= _output_get 7.5e+02)
        (if (== (Math|Random|RandomIntegerinRange 0 4) 0)
          (CallFunction|FarRange)
          (else
            (CallFunction|SeekPlayer)))
        (else
          (CallFunction|CloseRange))))))

(fn GetHealthasRatio
  (return (/ (Variables|Default|GetHealth) (Variables|Default|GetMaxHealth))))